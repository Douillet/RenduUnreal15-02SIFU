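; BP_CanBeKickedChair is a chair the player can kick away to knock down enemies.
; Overlap with a ThirdPersonCharacter toggles CanBeKick, which lets Projection push the Cube horizontally away from the first character's stored PlayerLocation and arm BringDownOpponnent.
; While armed, an overlapping actor that passes both the ThirdPersonCharacter and BP_Ennemy casts gets Fall called, then the chair disarms.
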(event Custom|Projection
  ;[1 1 1] Projection
  (if (Variables|Default|GetCanBeKick)
    (bind _outactors (Actor|GetAllActorsOfClass "/Game/ThirdPersonBP/Blueprints/ThirdPersonCharacter.ThirdPersonCharacter_C"))
    (Physics|AddForce (Variables|Actor|GetCube) (* (Math|Vector|Normalize (- (Transformation|GetWorldLocation (Variables|Actor|GetCube)) (Variables|/Game/ThirdPersonBP/Blueprints/ThirdPersonCharacter.ThirdPersonCharacter_C|GetPlayerLocation (Utilities|Array|Get(acopy) _outactors)))) "50000000.000000,50000000.000000,0.000000") "None" false)
    (Variables|Default|SetBringDownOpponnent true)))

(event Collision|EventActorBeginOverlap
  (params (OtherActor :type Actor%20Object%20Reference))
  ;[1 1 1] Player dans le trigger et peut Kicker la Chaise
  (Utilities|Casting|CastToThirdPersonCharacter OtherActor)
  (Variables|Default|SetCanBeKick true)
  ;[1 1 1] Touche un Ennemi
  (if (Variables|Default|GetBringDownOpponnent)
    (bind _asennemy (Utilities|Casting|CastToBP_Ennemy OtherActor))
    (Default|Fall _asennemy)
    (Variables|Default|SetBringDownOpponnent false)))

(event Collision|EventActorEndOverlap
  (params (OtherActor :type Actor%20Object%20Reference))
  ;[1 1 1] Player dans le trigger et peut Kicker la Chaise
  (Utilities|Casting|CastToThirdPersonCharacter OtherActor)
  (Variables|Default|SetCanBeKick false))

(fn ConstructionScript)